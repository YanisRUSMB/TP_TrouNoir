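; Black hole projectile actor that flies briefly, then stops and turns into a radial force field that destroys objects overlapping it.
; Timers started on BeginPlay drive it: one removes the sphere, activates the effect and opens a gate, another destroys the actor later.
; A fast looping timer feeds that gate to fire repeated radial impulses.
; While exploding, newly overlapping movable actors are destroyed, except Pawns.
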(event Custom|Delete
  (Actor|DestroyActor))

(event Custom|Explode
  (Components|DestroyComponent (Variables|Default|GetSphere))
  (Components|Activation|Activate (Variables|Default|GetBulletFX) false)
  (Components|Movement|StopMovementImmediately (Variables|Default|GetProjectileComponent))
  (Variables|Default|SetisExploding true)
  (Utilities|FlowControl|Gate true) ; enters at Open
)

(event Custom|Impluse
  (Utilities|FlowControl|Gate true
    (:Exit
      (Class|RadialForceComponent|FireImpulse (Variables|Default|GetRadialForce)))))

(event EventBeginPlay
  (Utilities|Time|SetTimerbyEvent (delegate Custom|Delete) 1e+01)
  (Utilities|Time|SetTimerbyEvent (delegate Custom|Explode) 3.0)
  (Utilities|Time|SetTimerbyEvent (delegate Custom|Impluse) 0.1 true))

(event Collision|EventActorBeginOverlap
  (params (OtherActor :type Actor%20Object%20Reference))
  (Utilities|Casting|CastToPawn OtherActor
    (:CastFailed
      (if (and (Variables|Default|GetisExploding) (Utilities|Enum|Equal(Enum) (Variables|/Script/Engine.SceneComponent|GetMobility (Variables|/Script/Engine.Actor|GetRootComponent OtherActor)) "Movable"))
        (Actor|DestroyActor OtherActor)))))

(fn ConstructionScript)